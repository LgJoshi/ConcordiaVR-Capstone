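; Parent Blueprint for sci-fi modular kitbash level elements, exposing per-instance material tinting on a base static mesh.
; The construction script pushes emissive power and color, four custom colors and a metallic color to the SMBaseMesh materials as named parameters.
; A boolean becomes a scalar isCustomColors parameter, passing the custom-color switch to the shader.
; The event graph holds only disabled stub events, so it has no runtime logic.
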(fn `UserConstructionScript`
  (bind _sm_basemesh (`self.SM_BaseMesh`))
  (bind _sm_basemesh_2 (`self.SM_BaseMesh`))
  (`|ExecutionSequence`
    (:`then_0`
      (`MeshComponent.SetScalarParameterValueOnMaterials` _sm_basemesh "EmissivePower" (`self.EmissivePower`)))
    (:`then_1`
      (`MeshComponent.SetVectorParameterValueOnMaterials` _sm_basemesh "EmissiveColor" (`KismetMathLibrary.Conv_LinearColorToVector` (`self.EmissiveColor`))))
    (:`then_2`
      (`MeshComponent.SetVectorParameterValueOnMaterials` _sm_basemesh_2 "Color01" (`KismetMathLibrary.Conv_LinearColorToVector` (`self.Color01`)))
      (`MeshComponent.SetVectorParameterValueOnMaterials` _sm_basemesh_2 "Color02" (`KismetMathLibrary.Conv_LinearColorToVector` (`self.Color02`)))
      (`MeshComponent.SetVectorParameterValueOnMaterials` _sm_basemesh_2 "Color03" (`KismetMathLibrary.Conv_LinearColorToVector` (`self.Color03`)))
      (`MeshComponent.SetVectorParameterValueOnMaterials` _sm_basemesh_2 "Color04" (`KismetMathLibrary.Conv_LinearColorToVector` (`self.Color04`)))
      (`MeshComponent.SetVectorParameterValueOnMaterials` _sm_basemesh_2 "MetallicColor" (`KismetMathLibrary.Conv_LinearColorToVector` (`self.ColorMetallic`))))
    (:`then_3`
      (`MeshComponent.SetScalarParameterValueOnMaterials` (`self.SM_BaseMesh`) "isCustomColors" (`KismetMathLibrary.Conv_BoolToDouble` (`self.isCustomColors`))))))