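; BP_Door01 is a configurable sci-fi sliding door that opens when something enters its OpenCollision and closes when it leaves.
; The overlaps play or reverse the DoorOpening timeline with sounds, and its track drives OpenPercent, which DoorPosition turns into a clamped X offset, optionally reversed.
; The construction script previews that position, toggles lights and walls, and pushes custom colors and emissive settings to mesh materials and lights.
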(event `self.OpenCollision.OnComponentBeginOverlap`
  (params (OverlappedComponent :type "PrimitiveComponent Object Reference") (OtherActor :type "Actor Object Reference") (OtherComp :type "PrimitiveComponent Object Reference") (OtherBodyIndex :type Integer) (bFromSweep :type Boolean) (SweepResult :type "HitResult Structure (by ref)"))
  (if (`self.isDoorClosed`)
    (`TimelineComponent.Play` (`self.DoorOpening`))
    (set `self.isDoorClosed` false)
    ;[1 1 1] PlayOpenSound
    (`GameplayStatics.PlaySoundAtLocation` "/Game/SciFi_Modular_Kitbash_Level/Sounds/SC_DoorSlidingOpening.SC_DoorSlidingOpening" (`SceneComponent.K2_GetComponentLocation` (`self.SM_Door01`)) (struct) 1.0 1.0 0.0 null null null)))

(event `self.OpenCollision.OnComponentEndOverlap`
  (params (OverlappedComponent :type "PrimitiveComponent Object Reference") (OtherActor :type "Actor Object Reference") (OtherComp :type "PrimitiveComponent Object Reference") (OtherBodyIndex :type Integer))
  (if (not (`self.isDoorClosed`))
    (`TimelineComponent.Reverse` (`self.DoorOpening`))
    (set `self.isDoorClosed` true)
    (`GameplayStatics.PlaySoundAtLocation` "/Game/SciFi_Modular_Kitbash_Level/Sounds/SC_DoorSlidingClosing.SC_DoorSlidingClosing" (`SceneComponent.K2_GetComponentLocation` (`self.SM_Door01`)) (struct) 1.0 1.0 0.0 null null null)))

(fn `DoorPosition`
  (bind _returnvalue (`KismetMathLibrary.FClamp` (* (`self.OpenPercent`) 1.3) 0.0 130.0))
  (`SceneComponent.K2_SetRelativeLocation` (`self.SM_Door01`) (`KismetMathLibrary.MakeVector` (select `bool` (`self.isOpenReverse`) :`false` _returnvalue :`true` (* -1 _returnvalue))) false false))

(fn `UserConstructionScript`
  (bind _sm_framebase (`self.SM_FrameBase`))
  (`|ExecutionSequence`
    (:`then_0`
      (`SceneComponent.SetVisibility` (`self.Light01`) (`self.EnableLight`) false)
      (`SceneComponent.SetVisibility` (`self.Light02`) (`self.EnableLight`) false))
    (:`then_1`
      (`self.DoorPosition`))
    (:`then_2`
      (`SceneComponent.SetVisibility` (`self.SM_DoorsWall01`) (`self.isWallVisible`) false)
      (`SceneComponent.SetVisibility` (`self.SM_DoorsWall02`) (`self.isWallVisible`) false))
    (:`then_3`
      (`|ExecutionSequence`
        (:`then_0`
          (`MeshComponent.SetScalarParameterValueOnMaterials` (`self.SM_FrameBase`) "EmissivePower" (`self.EmissicePower`))
          (`MeshComponent.SetScalarParameterValueOnMaterials` (`self.SM_Door01`) "EmissivePower" (`self.EmissicePower`))
          (`MeshComponent.SetScalarParameterValueOnMaterials` (`self.SM_FrameMiddle`) "EmissivePower" (`self.EmissicePower`))
          (`MeshComponent.SetScalarParameterValueOnMaterials` (`self.SM_FrameBase02`) "EmissivePower" (`self.EmissicePower`))
          (`MeshComponent.SetScalarParameterValueOnMaterials` (`self.SM_DoorsWall01`) "EmissivePower" (`self.EmissicePower`))
          (`MeshComponent.SetScalarParameterValueOnMaterials` (`self.SM_DoorsWall02`) "EmissivePower" (`self.EmissicePower`))
          (`MeshComponent.SetVectorParameterValueOnMaterials` (`self.SM_DoorsWall02`) "EmissiveColor" (`KismetMathLibrary.Conv_LinearColorToVector` (`self.EmissiveColor`)))
          (`MeshComponent.SetVectorParameterValueOnMaterials` (`self.SM_DoorsWall01`) "EmissiveColor" (`KismetMathLibrary.Conv_LinearColorToVector` (`self.EmissiveColor`)))
          (`MeshComponent.SetVectorParameterValueOnMaterials` (`self.SM_FrameBase02`) "EmissiveColor" (`KismetMathLibrary.Conv_LinearColorToVector` (`self.EmissiveColor`)))
          (`MeshComponent.SetVectorParameterValueOnMaterials` (`self.SM_FrameMiddle`) "EmissiveColor" (`KismetMathLibrary.Conv_LinearColorToVector` (`self.EmissiveColor`)))
          (`MeshComponent.SetVectorParameterValueOnMaterials` (`self.SM_Door01`) "EmissiveColor" (`KismetMathLibrary.Conv_LinearColorToVector` (`self.EmissiveColor`)))
          (`MeshComponent.SetVectorParameterValueOnMaterials` (`self.SM_FrameBase`) "EmissiveColor" (`KismetMathLibrary.Conv_LinearColorToVector` (`self.EmissiveColor`))))
        (:`then_1`
          (`MeshComponent.SetVectorParameterValueOnMaterials` _sm_framebase "Color01" (`KismetMathLibrary.Conv_LinearColorToVector` (`self.Color01`)))
          (`MeshComponent.SetVectorParameterValueOnMaterials` (`self.SM_Door01`) "Color01" (`KismetMathLibrary.Conv_LinearColorToVector` (`self.Color01`)))
          (`MeshComponent.SetVectorParameterValueOnMaterials` (`self.SM_FrameMiddle`) "Color01" (`KismetMathLibrary.Conv_LinearColorToVector` (`self.Color01`)))
          (`MeshComponent.SetVectorParameterValueOnMaterials` (`self.SM_FrameBase02`) "Color01" (`KismetMathLibrary.Conv_LinearColorToVector` (`self.Color01`)))
          (`MeshComponent.SetVectorParameterValueOnMaterials` (`self.SM_DoorsWall01`) "Color01" (`KismetMathLibrary.Conv_LinearColorToVector` (`self.Color01`)))
          (`MeshComponent.SetVectorParameterValueOnMaterials` (`self.SM_DoorsWall02`) "Color01" (`KismetMathLibrary.Conv_LinearColorToVector` (`self.Color01`)))
          (`MeshComponent.SetVectorParameterValueOnMaterials` _sm_framebase "Color02" (`KismetMathLibrary.Conv_LinearColorToVector` (`self.Color02`)))
          (`MeshComponent.SetVectorParameterValueOnMaterials` (`self.SM_Door01`) "Color02" (`KismetMathLibrary.Conv_LinearColorToVector` (`self.Color02`)))
          (`MeshComponent.SetVectorParameterValueOnMaterials` (`self.SM_FrameMiddle`) "Color02" (`KismetMathLibrary.Conv_LinearColorToVector` (`self.Color02`)))
          (`MeshComponent.SetVectorParameterValueOnMaterials` (`self.SM_FrameBase02`) "Color02" (`KismetMathLibrary.Conv_LinearColorToVector` (`self.Color02`)))
          (`MeshComponent.SetVectorParameterValueOnMaterials` (`self.SM_DoorsWall02`) "Color02" (`KismetMathLibrary.Conv_LinearColorToVector` (`self.Color02`)))
          (`MeshComponent.SetVectorParameterValueOnMaterials` (`self.SM_DoorsWall01`) "Color02" (`KismetMathLibrary.Conv_LinearColorToVector` (`self.Color02`)))
          (`MeshComponent.SetVectorParameterValueOnMaterials` _sm_framebase "Color03" (`KismetMathLibrary.Conv_LinearColorToVector` (`self.Color03`)))
          (`MeshComponent.SetVectorParameterValueOnMaterials` (`self.SM_Door01`) "Color03" (`KismetMathLibrary.Conv_LinearColorToVector` (`self.Color03`)))
          (`MeshComponent.SetVectorParameterValueOnMaterials` (`self.SM_FrameMiddle`) "Color03" (`KismetMathLibrary.Conv_LinearColorToVector` (`self.Color03`)))
          (`MeshComponent.SetVectorParameterValueOnMaterials` (`self.SM_FrameBase02`) "Color03" (`KismetMathLibrary.Conv_LinearColorToVector` (`self.Color03`)))
          (`MeshComponent.SetVectorParameterValueOnMaterials` (`self.SM_DoorsWall01`) "Color03" (`KismetMathLibrary.Conv_LinearColorToVector` (`self.Color03`)))
          (`MeshComponent.SetVectorParameterValueOnMaterials` (`self.SM_DoorsWall02`) "Color03" (`KismetMathLibrary.Conv_LinearColorToVector` (`self.Color03`)))
          (`MeshComponent.SetVectorParameterValueOnMaterials` (`self.SM_DoorsWall02`) "Color04" (`KismetMathLibrary.Conv_LinearColorToVector` (`self.Color04`)))
          (`MeshComponent.SetVectorParameterValueOnMaterials` (`self.SM_DoorsWall01`) "Color04" (`KismetMathLibrary.Conv_LinearColorToVector` (`self.Color04`)))
          (`MeshComponent.SetVectorParameterValueOnMaterials` (`self.SM_FrameBase02`) "Color04" (`KismetMathLibrary.Conv_LinearColorToVector` (`self.Color04`)))
          (`MeshComponent.SetVectorParameterValueOnMaterials` (`self.SM_FrameMiddle`) "Color04" (`KismetMathLibrary.Conv_LinearColorToVector` (`self.Color04`)))
          (`MeshComponent.SetVectorParameterValueOnMaterials` (`self.SM_Door01`) "Color04" (`KismetMathLibrary.Conv_LinearColorToVector` (`self.Color04`)))
          (`MeshComponent.SetVectorParameterValueOnMaterials` _sm_framebase "Color04" (`KismetMathLibrary.Conv_LinearColorToVector` (`self.Color04`)))
          (`MeshComponent.SetVectorParameterValueOnMaterials` _sm_framebase "MetallicColor" (`KismetMathLibrary.Conv_LinearColorToVector` (`self.ColorMetallic`)))
          (`MeshComponent.SetVectorParameterValueOnMaterials` (`self.SM_Door01`) "MetallicColor" (`KismetMathLibrary.Conv_LinearColorToVector` (`self.ColorMetallic`)))
          (`MeshComponent.SetVectorParameterValueOnMaterials` (`self.SM_FrameMiddle`) "MetallicColor" (`KismetMathLibrary.Conv_LinearColorToVector` (`self.ColorMetallic`)))
          (`MeshComponent.SetVectorParameterValueOnMaterials` (`self.SM_FrameBase02`) "MetallicColor" (`KismetMathLibrary.Conv_LinearColorToVector` (`self.ColorMetallic`)))
          (`MeshComponent.SetVectorParameterValueOnMaterials` (`self.SM_DoorsWall01`) "MetallicColor" (`KismetMathLibrary.Conv_LinearColorToVector` (`self.ColorMetallic`)))
          (`MeshComponent.SetVectorParameterValueOnMaterials` (`self.SM_DoorsWall02`) "MetallicColor" (`KismetMathLibrary.Conv_LinearColorToVector` (`self.ColorMetallic`))))
        (:`then_2`
          (`MeshComponent.SetScalarParameterValueOnMaterials` (`self.SM_DoorsWall02`) "isCustomColors" (`KismetMathLibrary.Conv_BoolToDouble` (`self.isCustomColor`)))
          (`MeshComponent.SetScalarParameterValueOnMaterials` (`self.SM_DoorsWall01`) "isCustomColors" (`KismetMathLibrary.Conv_BoolToDouble` (`self.isCustomColor`)))
          (`MeshComponent.SetScalarParameterValueOnMaterials` (`self.SM_FrameBase02`) "isCustomColors" (`KismetMathLibrary.Conv_BoolToDouble` (`self.isCustomColor`)))
          (`MeshComponent.SetScalarParameterValueOnMaterials` (`self.SM_FrameMiddle`) "isCustomColors" (`KismetMathLibrary.Conv_BoolToDouble` (`self.isCustomColor`)))
          (`MeshComponent.SetScalarParameterValueOnMaterials` (`self.SM_Door01`) "isCustomColors" (`KismetMathLibrary.Conv_BoolToDouble` (`self.isCustomColor`)))
          (`MeshComponent.SetScalarParameterValueOnMaterials` (`self.SM_FrameBase`) "isCustomColors" (`KismetMathLibrary.Conv_BoolToDouble` (`self.isCustomColor`))))
        (:`then_3`
          (`LightComponent.SetIntensity` (`self.Light02`) (`self.EmissicePower`))
          (`LightComponent.SetIntensity` (`self.Light01`) (`self.EmissicePower`))
          (`LightComponent.SetLightColor` (`self.Light01`) (`self.EmissiveColor`) true)
          (`LightComponent.SetLightColor` (`self.Light02`) (`self.EmissiveColor`) true))))))