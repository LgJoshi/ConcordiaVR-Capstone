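; BP_Column02 is a column Blueprint from the sci-fi modular kitbash level with an optional, configurable light.
; The construction script sets Light1's visibility from EnableLight, then copies the intensity and color of the Light component onto Light1.
; Only the visibility of Light1 is toggled, without propagating to children.
; The event graph holds only disabled default events, so it adds no runtime logic.
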(fn `UserConstructionScript`
  (bind _light1 (`self.Light1`))
  (bind _light (`self.Light`))
  (`parent.UserConstructionScript`)
  (`|ExecutionSequence`
    (:`then_0`
      (`SceneComponent.SetVisibility` (`self.Light1`) (`self.EnableLight`) false))
    (:`then_1`
      (`LightComponent.SetIntensity` _light1 (`LightComponentBase.Intensity` _light))
      (`LightComponent.SetLightColor` _light1 (`LightComponentBase.GetLightColor` _light) true))))