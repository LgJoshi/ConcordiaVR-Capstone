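; BP_SciFI_ElementLightParent is a base Blueprint for light-bearing elements in the SciFi Modular Kitbash level kit.
; Its construction script sets the Light component's visibility from EnableLight, then drives its intensity from EmissivePower and its color from EmissiveColor.
; The event graph adds no runtime logic, only a parent Tick call and disabled default events.
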(event `self.ReceiveTick`
  (params (DeltaSeconds :type "Float (single-precision)"))
  (`parent.ReceiveTick` DeltaSeconds))

(fn `UserConstructionScript`
  (bind _light (`self.Light`))
  (`parent.UserConstructionScript`)
  (`|ExecutionSequence`
    (:`then_0`
      (`SceneComponent.SetVisibility` (`self.Light`) (`self.EnableLight`) false))
    (:`then_1`
      (`LightComponent.SetIntensity` _light (`self.EmissivePower`))
      (`LightComponent.SetLightColor` _light (`self.EmissiveColor`) true))))