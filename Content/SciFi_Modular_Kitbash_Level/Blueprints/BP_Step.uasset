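; BP_Step is a modular staircase actor that builds a run of steps from a configurable count in its construction script.
; It adds copies of StepMesh's static mesh, each placed relative to the previous one by a horizontal Y offset and fixed vertical rise.
; The original and generated steps then receive two color parameters and a custom-color toggle on their materials.
; The event graph holds no active logic.
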(fn `UserConstructionScript`
  (bind _newstepcomponents (`self.NewStepComponents`))
  (`|ExecutionSequence`
    (:`then_0`
      (`KismetArrayLibrary.Array_Clear` (`self.NewStepComponents`))
      (for _index (range (+ (- (`self.StepsCount`) 2) 1))
        (bind _returnvalue_location (`KismetMathLibrary.BreakTransform` (`SceneComponent.GetRelativeTransform` (`|GetArrayItem` (`self.NewStepComponents`) (- _index 1)))))
        (bind _returnvalue (`AddComponent|NODE_AddStaticMeshComponent-0` :`RelativeTransform` (`KismetMathLibrary.Conv_VectorToTransform` (`KismetMathLibrary.MakeVector` (.x _returnvalue_location) (- (.y _returnvalue_location) (`self.NextStepHorizontalOffset`)) (+ (.z _returnvalue_location) 15.0)))))
        (`StaticMeshComponent.SetStaticMesh` _returnvalue (`StaticMeshComponent.StaticMesh` (`self.StepMesh`)))
        (`KismetArrayLibrary.Array_Add` (`self.NewStepComponents`) _returnvalue)))
    (:`then_1`
      (`KismetArrayLibrary.Array_Add` (`self.NewStepComponents`) (`self.StepMesh`)))
    (:`then_3`
      (`MeshComponent.SetVectorParameterValueOnMaterials` _newstepcomponents "Color01" (`KismetMathLibrary.Conv_LinearColorToVector` (`self.Color01`)))
      (`MeshComponent.SetVectorParameterValueOnMaterials` _newstepcomponents "Color02" (`KismetMathLibrary.Conv_LinearColorToVector` (`self.Color02`))))
    (:`then_4`
      (`MeshComponent.SetScalarParameterValueOnMaterials` _newstepcomponents "isCustomColors" (`KismetMathLibrary.Conv_BoolToDouble` (`self.isCustomColors`))))))