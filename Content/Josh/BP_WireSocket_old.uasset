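; VR wire socket that, when grabbed, starts a cable connection intended for its partner socket.
; Pickup spawns a BP_WirePickup on the grabbing motion controller, gives it origin and target sockets, and adds a cable component.
; AttachCable_Event pins the cable end to the partner and marks the socket active, while FailCable_Event destroys the cable.
; The line-trace logic meant to make the cable follow the hand is disconnected and never runs.
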(event `self.ReceiveTick`
  (params (DeltaSeconds :type "Float (single-precision)"))
  ;[1 1 1] Make the cable appear to follow the grabbing hand
)

(event `/Game/Blueprints/PickupActorInterface.Pickup`
  (params (AttachTo :type "SceneComponent Object Reference") (MotionController :type "MotionControllerComponent Object Reference"))
  (bind _output_get (set `self.CurrentMotionController` AttachTo))
  (bind _returnvalue (`|SpawnActorFromClass` "/Game/Josh/BP_WirePickup.BP_WirePickup_C" (`KismetMathLibrary.MakeTransform` (0.0 0.0 0.0)) "Undefined" "OverrideRootScale" null null))
  ;[1 1 1] Set values of wire pickup
  (bind _output_get_2 (set `self.Spawned Pickup` _returnvalue))
  (`SceneComponent.K2_AttachToComponent` (`Actor.RootComponent` _output_get_2) _output_get "None" "KeepWorld" "KeepRelative" "KeepWorld" false)
  (bind _asbp_wire_pickup (cast `/Game/Josh/BP_WirePickup` _output_get_2))
  (set `/Game/Josh/BP_WirePickup.Origin Socket` self _asbp_wire_pickup)
  (set `/Game/Josh/BP_WirePickup.Target Socket` (`self.PartnerSocket`) _asbp_wire_pickup)
  (`KismetSystemLibrary.PrintString` "wire spawned in")
  (bind _returnvalue_2 (`|AddComponentByClass` "/Script/CableComponent.CableComponent"))
  (bind _output_get_3 (set `self.MyCable` _returnvalue_2))
  (set `CableComponent.CableLength` 30.0 _output_get_3)
  (set `CableComponent.CableWidth` 3.0 _output_get_3))

(event `AttachCable_Event`
  (bind _mycable (`self.MyCable`))
  (`/Engine/EditorBlueprintResources/StandardMacros.IsValid` _mycable
    (:`Is Valid`
      (`CableComponent.SetAttachEndTo` _mycable (`self.PartnerSocket`) "None" "None")
      (set `self.IsActive` true))))

(event `FailCable_Event`
  (`ActorComponent.K2_DestroyComponent` (`self.MyCable`)))

(fn `UserConstructionScript`)