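; Wind volume actor, apparently for a wind tunnel, that pushes slow-moving pickups along its forward direction.
; When a BP_Pickup or subclass begins overlapping the Box, its velocity is compared against MinimumSpeed.
; If it is slower, its static mesh receives one mass-dependent AddForce of WindPushForce along the root's forward vector.
; The force fires only on overlap begin, with no continuous push while inside.
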(event `self.Box.OnComponentBeginOverlap`
  (params (OverlappedComponent :type "PrimitiveComponent Object Reference") (OtherActor :type "Actor Object Reference") (OtherComp :type "PrimitiveComponent Object Reference") (OtherBodyIndex :type Integer) (bFromSweep :type Boolean) (SweepResult :type "HitResult Structure (by ref)"))
  (if (`KismetMathLibrary.ClassIsChildOf` (`GameplayStatics.GetObjectClass` OtherActor) "/Game/Blueprints/BP_Pickup.BP_Pickup_C")
    (if (< (`KismetMathLibrary.VSize` (`self.GetVelocity` OtherActor)) (`self.Minimum Speed`))
      (`PrimitiveComponent.AddForce` (`self.GetComponentByClass` OtherActor "/Script/Engine.StaticMeshComponent") (* (`SceneComponent.GetForwardVector` (`self.DefaultSceneRoot`)) (`self.WindPushForce`)) "None" false))))

(fn `UserConstructionScript`)