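; BP_WirePickup_old is a wire pickup actor for connecting a cable from an origin socket to a target socket.
; On Drop, it checks whether its static mesh is within DropoffDistance of the target socket.
; It then calls the attach or fail cable event on the origin BP_WireSocket and destroys itself, provided that cast succeeds.
; BeginPlay only prints a debug message.
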(event `self.ReceiveBeginPlay`
  (`parent.ReceiveBeginPlay`)
  (`KismetSystemLibrary.PrintString` "O\\, alive"))

(event `/Game/Blueprints/PickupActorInterface.Drop`
  (params (MotionController :type "MotionControllerComponent Object Reference"))
  (if (< (`KismetMathLibrary.Vector_Distance` (`SceneComponent.K2_GetComponentLocation` (`self.StaticMeshComponent`)) (`SceneComponent.K2_GetComponentLocation` (`Actor.RootComponent` (`self.Target Socket`)))) (`self.Dropoff Distance`))
    (bind _asbp_wire_socket (cast `/Game/Josh/BP_WireSocket` (`self.Origin Socket`)))
    (`/Game/Josh/BP_WireSocket.AttachCable_Event` _asbp_wire_socket)
    (else
      (bind _asbp_wire_socket_2 (cast `/Game/Josh/BP_WireSocket` (`self.Origin Socket`)))
      (`/Game/Josh/BP_WireSocket.FailCable_Event` _asbp_wire_socket_2)))
  (`self.K2_DestroyActor`))

(fn `UserConstructionScript`
  (`parent.UserConstructionScript`))