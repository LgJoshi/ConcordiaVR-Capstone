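; BP_WirePickup is a grabbable wire actor that BP_MotionController picks up, apparently meant to plug into a target socket.
; Pickup turns off mesh physics and attaches the root to the passed component, keeping world transform.
; Drop checks whether the mesh is within DropoffDistance of TargetSocket, then only casts OriginSocket to BP_WireSocket.
; Drop is unfinished: it neither detaches the actor, restores physics, nor makes a connection.
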(event `/Game/Blueprints/PickupActorInterface.Pickup`
  (params (AttachTo :type "SceneComponent Object Reference"))
  (`PrimitiveComponent.SetSimulatePhysics` (`self.StaticMeshComponent`) false)
  (`SceneComponent.K2_AttachToComponent` (`self.K2_GetRootComponent`) AttachTo "None" "KeepWorld" "KeepWorld" "KeepWorld" false))

(event `/Game/Blueprints/PickupActorInterface.Drop`
  (if (< (`KismetMathLibrary.Vector_Distance` (`SceneComponent.K2_GetComponentLocation` (`self.StaticMeshComponent`)) (`SceneComponent.K2_GetComponentLocation` (`Actor.RootComponent` (`self.Target Socket`)))) (`self.Dropoff Distance`))
    (cast `/Game/Josh/BP_WireSocket` (`self.Origin Socket`))))

(fn `UserConstructionScript`
  (`parent.UserConstructionScript`))