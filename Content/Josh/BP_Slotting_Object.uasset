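; BP_Slotting_Object is a carried puzzle piece that checks on Drop whether it fits its TargetSlotActor.
; After detaching, CheckRotationPosition compares Arrow-to-slot distance and per-axis forward-vector differences against error tolerances, printing debug values; roll is ignored.
; A match moves the slot actor, not the piece, to world origin and applies an emissive material; a miss enables physics.
; The attach-parent lookup for the target is unwired.
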(event `self.ReceiveBeginPlay`
  (`parent.ReceiveBeginPlay`)
  (`KismetSystemLibrary.PrintString` (`KismetStringLibrary.Concat_StrStr` "Target slot: " (`KismetSystemLibrary.GetObjectName` (`self.TargetSlotActor`)))))

(event `/Game/Blueprints/PickupActorInterface.Drop`
  (`self.K2_DetachFromActor` "KeepWorld" "KeepWorld" "KeepWorld")
  (bind _truefalse (`self.CheckRotationPosition`))
  (if _truefalse
    (`self.K2_SetActorLocation` (`self.TargetSlotActor`) (0.0 0.0 0.0) false false)
    (`PrimitiveComponent.SetMaterial` (`self.StaticMeshComponent`) 0 "/Game/SciFi_Modular_Kitbash_Level/Materials/MI_LightEmissive.MI_LightEmissive")
    (else
      (`PrimitiveComponent.SetSimulatePhysics` (`self.StaticMeshComponent`) true))))

(fn `CheckRotationPosition`
  (returns (TrueFalse :type Boolean))
  (bind _errorrotation (`self.ErrorRotation`))
  (bind _rootcomponent (`self.RootComponent`))
  (bind (_returnvalue_x _returnvalue_y _returnvalue_z) (`KismetMathLibrary.BreakVector` (`SceneComponent.GetForwardVector` _rootcomponent)))
  (bind _rootcomponent_2 (`Actor.RootComponent` (`self.TargetSlotActor`)))
  (bind (_returnvalue_x_2 _returnvalue_y_2 _returnvalue_z_2) (`KismetMathLibrary.BreakVector` (`SceneComponent.GetForwardVector` _rootcomponent_2)))
  (bind _returnvalue (`KismetMathLibrary.Abs` (- _returnvalue_x _returnvalue_x_2)))
  (bind _returnvalue_2 (`KismetMathLibrary.Abs` (- _returnvalue_y _returnvalue_y_2)))
  (bind _returnvalue_3 (`KismetMathLibrary.Abs` (- _returnvalue_z _returnvalue_z_2)))
  (`KismetSystemLibrary.PrintString` (`KismetStringLibrary.Concat_StrStr` "my forward: " (`KismetStringLibrary.Conv_VectorToString` (`SceneComponent.GetForwardVector` _rootcomponent))))
  (`KismetSystemLibrary.PrintString` (`KismetStringLibrary.Concat_StrStr` "slot forward: " (`KismetStringLibrary.Conv_VectorToString` (`SceneComponent.GetForwardVector` _rootcomponent_2))))
  (`KismetSystemLibrary.PrintString` (`KismetStringLibrary.Concat_StrStr` (`KismetStringLibrary.Conv_DoubleToString` _returnvalue) "&" (`KismetStringLibrary.Conv_DoubleToString` _returnvalue_2) "&" (`KismetStringLibrary.Conv_DoubleToString` _returnvalue_3)) true true (struct :`R` 1.0 :`G` 0.988649 :`B` 0.187166 :`A` 1.0))
  (return (and (< (`KismetMathLibrary.Vector_Distance` (`SceneComponent.K2_GetComponentLocation` (`self.Arrow`)) (`SceneComponent.K2_GetComponentLocation` (`Actor.RootComponent` (`self.TargetSlotActor`)))) (`self.ErrorDistance`)) (and (< _returnvalue _errorrotation) (< _returnvalue_2 _errorrotation) (< _returnvalue_3 _errorrotation)))))

(fn `UserConstructionScript`
  (`parent.UserConstructionScript`))