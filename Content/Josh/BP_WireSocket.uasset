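; BP_WireSocket is a grabbable VR wire socket that spawns a cable component when picked up by a motion controller.
; Pickup attaches the socket to the controller and creates the cable; Drop clears the controller and destroys the cable.
; While held, Tick line-traces to the controller with debug drawing and writes the hit location into the cable's end.
; Partner-socket distance and cable-attach logic exists but is disconnected.
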(event `self.ReceiveTick`
  (params (DeltaSeconds :type "Float (single-precision)"))
  (if (and (`KismetSystemLibrary.IsValid` (`self.CurrentMotionController`)) (`KismetSystemLibrary.IsValid` (`self.MyCable`)))
    (bind _outhit (`KismetSystemLibrary.LineTraceSingleForObjects` :`End` (`SceneComponent.K2_GetComponentLocation` (`self.CurrentMotionController`)) :`ObjectTypes` (`self.Object Types`) :`DrawDebugType` "ForDuration"))
    (set `CableComponent.EndLocation` (`.Location` (`GameplayStatics.BreakHitResult` _outhit)) (`self.MyCable`))))

(event `/Game/Blueprints/PickupActorInterface.Pickup`
  (params (AttachTo :type "SceneComponent Object Reference"))
  (bind _output_get (set `self.CurrentMotionController` AttachTo))
  (`SceneComponent.K2_AttachToComponent` (`self.RootComponent`) _output_get "None" "KeepWorld" "KeepWorld" "KeepWorld" false)
  (`KismetSystemLibrary.PrintString` "I\"M GRABED")
  (bind _returnvalue (`|AddComponentByClass` "/Script/CableComponent.CableComponent"))
  (bind _output_get_2 (set `self.MyCable` _returnvalue))
  (set `CableComponent.CableLength` 30.0 _output_get_2)
  (set `CableComponent.CableWidth` 3.0 _output_get_2))

(event `/Game/Blueprints/PickupActorInterface.Drop`
  (`KismetSystemLibrary.PrintString` "destroy everything")
  (set `self.CurrentMotionController` null)
  (`ActorComponent.K2_DestroyComponent` (`self.MyCable`)))

(fn `UserConstructionScript`)