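; Slot actor for an object-slotting mechanic that shows whether its paired object is correctly positioned and rotated.
; On BeginPlay it takes its first attached actor as that object.
; While that object overlaps the trigger sphere, Tick polls its CheckRotationPosition and switches Sphere1 between an emissive material and a wall material.
; Any end overlap, regardless of actor, stops checking and applies a cube material.
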(event `self.ReceiveBeginPlay`
  (bind _output_get (set `self.SlotObject` (`|GetArrayItem` (`self.GetAttachedActors` true))))
  (`KismetSystemLibrary.PrintString` (`KismetSystemLibrary.GetObjectName` _output_get)))

(event `self.ReceiveTick`
  (params (DeltaSeconds :type "Float (single-precision)"))
  (bind _slotobject (`self.SlotObject`))
  (if (and (`self.CheckingRotPos`) (`KismetSystemLibrary.IsValid` _slotobject) (`KismetMathLibrary.ClassIsChildOf` (`GameplayStatics.GetObjectClass` _slotobject) "/Game/Josh/BP_Slotting_Object.BP_Slotting_Object_C"))
    (bind _asbp_slotting_object (cast `/Game/Josh/BP_Slotting_Object` (`self.SlotObject`)))
    (bind _truefalse (`/Game/Josh/BP_Slotting_Object.CheckRotationPosition` _asbp_slotting_object))
    (if _truefalse
      (`PrimitiveComponent.SetMaterial` (`self.Sphere1`) 0 "/Game/SciFi_Modular_Kitbash_Level/Materials/M_LightEmissive_master.M_LightEmissive_master")
      (else
        (`PrimitiveComponent.SetMaterial` (`self.Sphere1`) 0 "/Game/SciFi_Modular_Kitbash_Level/Materials/MI_Wall01.MI_Wall01")))))

(event `self.Sphere.OnComponentBeginOverlap`
  (params (OverlappedComponent :type "PrimitiveComponent Object Reference") (OtherActor :type "Actor Object Reference") (OtherComp :type "PrimitiveComponent Object Reference") (OtherBodyIndex :type Integer) (bFromSweep :type Boolean) (SweepResult :type "HitResult Structure (by ref)"))
  (bind _slotobject (`self.SlotObject`))
  (if (and (== OtherActor _slotobject) (`KismetSystemLibrary.IsValid` _slotobject))
    (set `self.CheckingRotPos` true)
    (`PrimitiveComponent.SetMaterial` (`self.Sphere1`) 0 "/Game/SciFi_Modular_Kitbash_Level/Materials/MI_Wall01.MI_Wall01")))

(event `self.Sphere.OnComponentEndOverlap`
  (params (OverlappedComponent :type "PrimitiveComponent Object Reference") (OtherActor :type "Actor Object Reference") (OtherComp :type "PrimitiveComponent Object Reference") (OtherBodyIndex :type Integer))
  (set `self.CheckingRotPos` false)
  (`PrimitiveComponent.SetMaterial` (`self.Sphere1`) 0 "/Game/Geometry/Meshes/CubeMaterial.CubeMaterial"))

(fn `UserConstructionScript`)